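; BPBossEnemy is a boss enemy Blueprint that dies from a single overlap with a player bullet.
; On overlap with a BPBasicBullet it destroys the bullet, adds score through player 0's BPPlayerPawn, then destroys itself.
; Tick resets rotation to zero and sets location from the capsule's position plus a Movement offset, which a zero multiplier cancels out.
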(event `self.ReceiveBeginPlay`)

(event `self.ReceiveActorBeginOverlap`
  (params (OtherActor :type "Actor Object Reference"))
  (bind _asbpbasic_bullet (cast `/Game/BluePrint/BPBasicBullet` OtherActor))
  (`self.K2_DestroyActor` _asbpbasic_bullet)
  (bind _asbpplayer_pawn (cast `/Game/BluePrint/BPPlayerPawn` (`GameplayStatics.GetPlayerPawn` 0)))
  (`self.IncreaseScore` _asbpplayer_pawn 100)
  (`self.K2_DestroyActor`))

(event `self.ReceiveTick`
  (params (DeltaSeconds :type "Float (single-precision)"))
  (`self.SetActorRotation` (struct))
  (`self.K2_SetActorLocation` (+ (* (`self.Movement`) (* 0.0 100.0)) (`SceneComponent.K2_GetComponentLocation` (`self.Capsule`)))))

(fn `UserConstructionScript`)