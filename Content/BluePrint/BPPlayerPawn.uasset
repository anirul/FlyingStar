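; Player ship pawn for an auto-forward flying shooter that tracks score and a water resource used as ammo.
; Each tick, input axes tilt the mesh within capped angles and ease it back to zero when released.
; That yaw and pitch drive clamped lateral and vertical movement while X advances constantly.
; Holding fire spawns slightly scattered BPBasicBullet actors from the mesh every tick while water remains.
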(event EventBeginPlay)

(event Collision|EventActorBeginOverlap
  (params (OtherActor :type Actor%20Object%20Reference)))

(event EventTick
  (params (DeltaSeconds :type Float%20%28single-precision%29))
  (CallFunction|SetShipRotation DeltaSeconds)
  (CallFunction|SetShipMove DeltaSeconds)
  (if (Variables|Default|GetFireing)
    (CallFunction|FireProjectile (Variables|Default|GetProjectileScale) (Variables|Default|GetProjectileFront))))

(event Input|ActionEvents|InputActionFIreMainWeapon
  (:Pressed
    (Variables|Default|SetFireing true))
  (:Released
    (Variables|Default|SetFireing false)))

(fn ConstructionScript)

(fn CapValue
  (params (Input :type Float%20%28single-precision%29) (MaxCap :type Float%20%28single-precision%29) (MinCap :type Float%20%28single-precision%29))
  ;[1 1 1] Check upper bound
  (if (> Input MaxCap)
    ;[1 1 1] > Max -> Max
    (LocalVariables|Setoutput_value MaxCap)
    (else
      ;[1 1 1] Check lower bound
      (if (< Input MinCap)
        ;[1 1 1] < Min -> Min
        (LocalVariables|Setoutput_value MinCap)
        (else
          ;[1 1 1] Val
          (LocalVariables|Setoutput_value Input)))))
  (return (LocalVariables|Getoutput_value)))

(fn RotationAxis
  (params (InputAxis :type Float%20%28single-precision%29) (InputValue :type Float%20%28single-precision%29) (InputFactor :type Float%20%28single-precision%29))
  (if (== InputAxis 0.0)
    (bind _output (CallFunction|RotateCounter InputValue InputFactor))
    (LocalVariables|Setout_rotation _output)
    (else
      (bind _output_2 (CallFunction|CapValue (+ (* InputAxis InputFactor) InputValue) (Variables|Default|Getmax_rotation_angle) (Variables|Default|Getmin_rotation_angle)))
      (LocalVariables|Setout_rotation _output_2)))
  (return (LocalVariables|Getout_rotation)))

(fn RotateCounter
  (params (InputValue :type Float%20%28single-precision%29) (InputFactor :type Float%20%28single-precision%29))
  (if (> InputValue 0.0)
    (bind _output_get (LocalVariables|Setout (- InputValue InputFactor)))
    (if (> _output_get 0.0)
      _
      (else
        (LocalVariables|Setout 0.0 :!label _label)))
    (elif (< InputValue 0.0)
      (bind _output_get_2 (LocalVariables|Setout (+ InputValue InputFactor)))
      (if (< _output_get_2 0.0)
        _
        (else
          (goto _label)))
      (else
        (goto _label))))
  (return (LocalVariables|Getout)))

(fn SetShipRotation
  (params (deltaTime :type Float%20%28single-precision%29))
  (bind _output_get (Variables|Default|Setrotation_factor (* (Variables|Default|Getrotation_acceletation) deltaTime)))
  (bind _output_rotation (CallFunction|RotationAxis (Input|AxisValues|GetMoveHorizontal) (Variables|Default|Getrotation_yaw) _output_get))
  (bind _output_get_2 (Variables|Default|Setrotation_yaw _output_rotation))
  (bind _output_rotation_2 (CallFunction|RotationAxis (Input|AxisValues|GetMoveVertical) (Variables|Default|Getrotation_pitch) _output_get))
  (bind _output_get_3 (Variables|Default|Setrotation_pitch _output_rotation_2))
  (Transformation|SetRelativeRotation (Variables|Default|GetPlayerMesh) (Class|KismetMathLibrary|MakeRot _output_get_3 _output_get_2 0.0) false))

(fn SetShipMove
  (params (detlaTime :type Float%20%28single-precision%29))
  (bind _returnvalue (Transformation|GetActorLocation))
  (bind (_x _y _z) (Math|Vector|BreakVector _returnvalue))
  (bind _output_get (Variables|Default|Setmove_lateral_factor (* (Variables|Default|Getmove_lateral_acceleration) detlaTime)))
  (bind _output_get_2 (Variables|Default|Setmove_forward_factor (* (Variables|Default|Getmove_forward_acceleration) detlaTime)))
  (bind _output (CallFunction|CapValue (+ (* (Variables|Default|Getrotation_yaw) _output_get) _y) 5e+02 -5e+02))
  (bind _output_2 (CallFunction|CapValue (+ (* (Variables|Default|Getrotation_pitch) _output_get) _z) 7e+02 1.5e+02))
  (Transformation|SetActorLocation (Math|Vector|MakeVector (+ _output_get_2 _x) _output _output_2) true)
  (Development|PrintString (Utilities|String|ToString(Text) (Utilities|Text|FormatText "pos ({x}, {y}, {z})" (Utilities|Text|ToText(Float) (+ _output_get_2 _x) "HalfToEven") (Utilities|Text|ToText(Float) (+ (* (Variables|Default|Getrotation_yaw) _output_get) _y) "HalfToEven") (Utilities|Text|ToText(Float) (+ (* (Variables|Default|Getrotation_pitch) _output_get) _z) "HalfToEven"))) false))

(fn FireProjectile
  (params (InputScale :type Float%20%28single-precision%29) (InputFront :type Float%20%28single-precision%29))
  (bind _playermesh (Variables|Default|GetPlayerMesh))
  (bind _returnvalue (Transformation|GetWorldTransform _playermesh))
  (bind (_location _rotation) (Math|Transform|BreakTransform _returnvalue))
  (if (> (Variables|Default|GetWater) 0.0)
    (Game|SpawnActorfromClass "/Game/BluePrint/BPBasicBullet.BPBasicBullet_C" (Math|Transform|MakeTransform (+ (+ _location (* (Math|Vector|GetForwardVector _rotation) InputFront)) (* (Math|Random|RandomUnitVector) 1e+01)) _rotation (Math|Vector|MakeVector InputScale InputScale InputScale)) true 0 0)
    (Variables|Default|SetWater (- (Variables|Default|GetWater) (Variables|Default|GetFireWaterConsumption)))))

(fn GetScore
  (return (Variables|Default|GetScore)))

(fn GetWater
  (return (Variables|Default|GetWater)))

(fn IncreaseScore
  (params (InputScore :type Integer))
  (Variables|Default|SetScore (+ (Variables|Default|GetScore) InputScore)))

(fn IncreaseWater
  (params (InputWater :type Float%20%28single-precision%29))
  (bind _output (CallFunction|CapValue (+ (Variables|Default|GetWater) InputWater) 1.0 0.0))
  (Variables|Default|SetWater _output))

(fn DecreaseWater
  (params (InputDecrease :type Float%20%28single-precision%29))
  (bind _output (CallFunction|CapValue (- (Variables|Default|GetWater) InputDecrease) 1.0 0.0))
  (Variables|Default|SetWater _output))