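; BPFlyingKittler is an actor, apparently a shootable flying target, that reacts to hits from BPBasicBullet.
; Each tick it moves without sweep by its Movement vector scaled by delta time, which starts at zero on BeginPlay and is not changed in this graph.
; An overlapping bullet is destroyed and switches on physics simulation for the CollisionSphere.
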(event `self.ReceiveBeginPlay`
  (set `self.Movement` (0.0 0.0 0.0)))

(event `self.ReceiveActorBeginOverlap`
  (params (OtherActor :type "Actor Object Reference"))
  (bind _asbpbasic_bullet (cast `/Game/BluePrint/BPBasicBullet` OtherActor))
  (`self.K2_DestroyActor` _asbpbasic_bullet)
  (`PrimitiveComponent.SetSimulatePhysics` (`self.CollisionSphere`) true))

(event `self.ReceiveTick`
  (params (DeltaSeconds :type "Float (single-precision)"))
  (`self.K2_SetActorLocation` (+ (* (`self.Movement`) (* DeltaSeconds 100.0)) (`SceneComponent.K2_GetComponentLocation` (`self.CollisionSphere`)))))

(fn `UserConstructionScript`)