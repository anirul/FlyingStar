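; BPStraitTile is a floor tile for an endlessly extending track, exposing an attach point transform for chaining.
; When the player pawn leaves its box, it asks BPGameMode to add a tile, then destroys itself two seconds later.
; SpawnEnemy always spawns a randomly offset flying enemy, adds three static enemies on Walker entries in the cyclic SpawnOrder, and returns the incremented index.
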(event `self.ReceiveBeginPlay`)

(event `self.ReceiveActorBeginOverlap`
  (params (OtherActor :type "Actor Object Reference")))

(event `self.ReceiveTick`
  (params (DeltaSeconds :type "Float (single-precision)")))

(event `self.Box.OnComponentEndOverlap`
  (params (OtherActor :type "Actor Object Reference") (OtherComp :type "PrimitiveComponent Object Reference") (OtherBodyIndex :type Integer))
  (cast `/Game/BluePrint/BPPlayerPawn` OtherActor)
  (bind _asbpgame_mode (cast `/Game/BluePrint/BPGameMode` (`GameplayStatics.GetGameMode`)))
  (`/Game/BluePrint/BPGameMode.AddFloorTile` _asbpgame_mode)
  (`KismetSystemLibrary.Delay` 2.0)
  (`self.K2_DestroyActor`))

(fn `GetAttachTransform`
  (returns (OutputAttachPoint :type "Transform Structure"))
  (return (`SceneComponent.K2_GetComponentToWorld` (`self.AttachPoint`))))

(fn `SpawnEnemy`
  (params (PreviousIndex :type Integer))
  (returns (NextIndex :type Integer))
  (bind _spawnorder (`self.SpawnOrder`))
  (bind _returnvalue (`SceneComponent.K2_GetComponentLocation` (`self.AttachPoint`)))
  ;[1 1 1] Bird Spawning
  (`|SpawnActorFromClass` "/Game/BluePrint/BPFlyingEnemy.BPFlyingEnemy_C" (`KismetMathLibrary.MakeTransform` (+ _returnvalue (`KismetMathLibrary.MakeVector` 0.0 (`KismetMathLibrary.RandomFloatInRange` -500.0 500.0) (`KismetMathLibrary.RandomFloatInRange` 200.0 500.0)))))
  (switch `/Game/BluePrint/BPSpawnTypeEnum` (`KismetArrayLibrary.Array_Get` _spawnorder (mod PreviousIndex (`KismetArrayLibrary.Array_Length` _spawnorder)))
    (:`NewEnumerator0`
      _)
    (:`NewEnumerator1`
      _)
    (:`NewEnumerator2`
      ;[1 1 1] Walker Init
      (`|SpawnActorFromClass` "/Game/BluePrint/BPStaticEnemy.BPStaticEnemy_C" (`KismetMathLibrary.MakeTransform` (+ _returnvalue (0.0 0.0 0.0))))
      (`|SpawnActorFromClass` "/Game/BluePrint/BPStaticEnemy.BPStaticEnemy_C" (`KismetMathLibrary.MakeTransform` (+ _returnvalue (0.0 -200.0 0.0))))
      (`|SpawnActorFromClass` "/Game/BluePrint/BPStaticEnemy.BPStaticEnemy_C" (`KismetMathLibrary.MakeTransform` (+ _returnvalue (0.0 200.0 0.0)))))
    (:`NewEnumerator3`
      _)
    (:`NewEnumerator4`
      _))
  (return (+ PreviousIndex 1)))

(fn `UserConstructionScript`)