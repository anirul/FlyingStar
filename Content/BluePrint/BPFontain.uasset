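; BPFontain is a temporary fountain actor that refills the player's water while the player stands near it.
; Sphere overlap events set a PlayerOverlap flag when a BPPlayerPawn enters or leaves.
; While the flag is set, Tick calls IncreaseWater on the player 0 pawn, scaled by delta time.
; BeginPlay starts a two-minute delay, after which the fountain destroys itself.
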(event `self.ReceiveBeginPlay`
  (`KismetSystemLibrary.Delay` 120.0)
  (`self.K2_DestroyActor`))

(event `self.ReceiveActorBeginOverlap`
  (params (OtherActor :type "Actor Object Reference")))

(event `self.ReceiveTick`
  (params (DeltaSeconds :type "Float (single-precision)"))
  (if (`self.PlayerOverlap`)
    (bind _asbpplayer_pawn (cast `/Game/BluePrint/BPPlayerPawn` (`GameplayStatics.GetPlayerPawn` 0)))
    (`/Game/BluePrint/BPPlayerPawn.IncreaseWater` _asbpplayer_pawn (* DeltaSeconds 1.0))))

(event `self.Sphere.OnComponentBeginOverlap`
  (params (OtherActor :type "Actor Object Reference") (OtherComp :type "PrimitiveComponent Object Reference") (OtherBodyIndex :type Integer) (bFromSweep :type Boolean) (SweepResult :type "HitResult Structure (by ref)"))
  (cast `/Game/BluePrint/BPPlayerPawn` OtherActor)
  (set `self.PlayerOverlap` true))

(event `self.Sphere.OnComponentEndOverlap`
  (params (OtherActor :type "Actor Object Reference") (OtherComp :type "PrimitiveComponent Object Reference") (OtherBodyIndex :type Integer))
  (cast `/Game/BluePrint/BPPlayerPawn` OtherActor)
  (set `self.PlayerOverlap` false))

(fn `UserConstructionScript`)