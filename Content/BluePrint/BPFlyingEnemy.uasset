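; Flying enemy actor that drifts along negative X with a slight random Y offset, moved each Tick by setting its location.
; A hit from a BPBasicBullet (which it destroys) or the player pawn, which also randomizes its rotation, triggers a one-time death.
; Death stops movement, enables physics on CollisionSphere, awards score and spawns an explosion.
; Dropping below world Z zero spawns another explosion, prints a debug string and destroys the actor.
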(event `self.ReceiveBeginPlay`
  (set `self.Movement` (`KismetMathLibrary.MakeVector` -5.0 (`KismetMathLibrary.RandomFloatInRange` -0.1 0.1))))

(event `self.ReceiveActorBeginOverlap`
  (params (OtherActor :type "Actor Object Reference"))
  (bind _asbpbasic_bullet (cast `/Game/BluePrint/BPBasicBullet` OtherActor)
    (:`then`
      (`self.K2_DestroyActor` _asbpbasic_bullet))
    (:`CastFailed`
      (cast `/Game/BluePrint/BPPlayerPawn` OtherActor)
      (`self.SetActorRotation` (`KismetMathLibrary.RandomRotator` false))))
  (if (not (`SceneComponent.IsSimulatingPhysics` (`self.CollisionSphere`) "None"))
    (`PrimitiveComponent.SetSimulatePhysics` (`self.CollisionSphere`) true)
    (set `self.Movement` (0.0 0.0 0.0))
    (bind _asbpplayer_pawn (cast `/Game/BluePrint/BPPlayerPawn` (`GameplayStatics.GetPlayerPawn` 0)))
    (`/Game/BluePrint/BPPlayerPawn.IncreaseScore` _asbpplayer_pawn 1000000)
    (`GameplayStatics.SpawnEmitterAtLocation` "/Game/Particule/P_Explosion.P_Explosion" (`SceneComponent.K2_GetComponentLocation` (`self.CollisionSphere`)))))

(event `self.ReceiveTick`
  (params (DeltaSeconds :type "Float (single-precision)"))
  (bind _returnvalue (`SceneComponent.K2_GetComponentLocation` (`self.CollisionSphere`)))
  (`self.K2_SetActorLocation` (+ (* (`self.Movement`) (* DeltaSeconds 100.0)) _returnvalue))
  (if (< (.z _returnvalue) 0.0)
    (`GameplayStatics.SpawnEmitterAtLocation` "/Game/Particule/P_Explosion.P_Explosion" _returnvalue)
    (`KismetSystemLibrary.PrintString` "Prout")
    (`self.K2_DestroyActor`)))

(fn `UserConstructionScript`)