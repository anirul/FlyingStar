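; BPGameMode is a game mode that builds a chain of ten floor tiles at BeginPlay.
; AddFloorTile spawns a BPStraitTile at NextSpawnPoint, then takes that tile's attach transform as the next spawn point.
; Each tile's SpawnEnemy receives NextIndex and returns the value for the following tile.
; The BPUserInterface widget is created and added to the viewport inside the same loop, so ten copies appear and UIReference keeps the last.
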(event `self.ReceiveBeginPlay`
  (for _ (range 10)
    (`self.AddFloorTile`)
    (bind _returnvalue (`|CreateWidget` "/Game/BluePrint/BPUserInterface.BPUserInterface_C"))
    (bind _output_get (set `self.UIReference` _returnvalue))
    (`UserWidget.AddToViewport` _output_get 0)))

(event `self.ReceiveTick`
  (params (DeltaSeconds :type "Float (single-precision)")))

(fn `AddFloorTile`
  (bind _returnvalue (`|SpawnActorFromClass` "/Game/BluePrint/BPStraitTile.BPStraitTile_C" (`self.NextSpawnPoint`)))
  (bind _nextindex (`/Game/BluePrint/BPStraitTile.SpawnEnemy` _returnvalue (`self.NextIndex`)))
  (set `self.NextIndex` _nextindex)
  (bind _outputattachpoint (`/Game/BluePrint/BPStraitTile.GetAttachTransform` _returnvalue))
  (set `self.NextSpawnPoint` _outputattachpoint))

(fn `UserConstructionScript`)